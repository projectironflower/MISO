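; BP_Puzzle_ is an actor Blueprint that hosts a puzzle UI widget and handles keyboard control for it.
; On BeginPlay it enables input for the first player controller and creates a WBP_Puzzle widget.
; The 3 key toggles the widget on and off the viewport along with the mouse cursor via FlipFlop.
; The U key calls the widget's Move function.
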(event `self.ReceiveBeginPlay`
  (`self.EnableInput` (`GameplayStatics.GetPlayerController` 0))
  (bind _returnvalue (`|CreateWidget` "/Game/Asset/Widget/WBP_Puzzle.WBP_Puzzle_C"))
  (set `self.Puzzle` _returnvalue))

(event `Key|Three`
  (params (Key :type "Key Structure"))
  (bind _returnvalue (`GameplayStatics.GetPlayerController` 0))
  (bind _puzzle (`self.Puzzle`))
  (:`Pressed`
    (`/Engine/EditorBlueprintResources/StandardMacros.FlipFlop`
      (:`A`
        (`UserWidget.AddToViewport` _puzzle 0)
        (set `PlayerController.bShowMouseCursor` true _returnvalue))
      (:`B`
        (`Widget.RemoveFromParent` _puzzle)
        (set `PlayerController.bShowMouseCursor` false _returnvalue)))))

(event `Key|U`
  (params (Key :type "Key Structure"))
  (:`Pressed`
    (`/Game/Asset/Widget/WBP_Puzzle.Move` (`self.Puzzle`))))

(fn `UserConstructionScript`)