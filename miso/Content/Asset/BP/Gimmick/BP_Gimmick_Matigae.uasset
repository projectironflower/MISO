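; BP_Gimmick_Matigae is a gimmick actor named "matigae" that clears in response to an event from a Guide.
; BeginPlay sets its name, and Get_Guid stores the Guide and binds a handler to its MatigaeCl dispatcher.
; That handler calls Clear, while Reset_Guid removes the binding.
; The Set_Debug function is empty, with leftover, unreachable nodes for setting debug widget text.
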(event `self.ReceiveBeginPlay`
  (`parent.ReceiveBeginPlay`)
  (set `self.Name` "matigae"))

(event `カスタムイベント_0`
  (`self.Clear`))

(event `Get_Guid`
  (params (Guide :type "/Game/Asset/BP/BP_Guide Object Reference"))
  (bind _output_get (set `self.Guide` Guide))
  (add `/Game/Asset/BP/BP_Guide.matigae_Cl` _output_get (delegate `カスタムイベント_0`)))

(event `Reset_Guid`
  (remove `/Game/Asset/BP/BP_Guide.matigae_Cl` (`self.Guide`) (delegate `カスタムイベント_0`)))

(fn `Set_Debug`)

(fn `UserConstructionScript`
  (`parent.UserConstructionScript`))