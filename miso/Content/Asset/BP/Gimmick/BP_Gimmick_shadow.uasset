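; BP_Gimmick_shadow is a shadow gimmick (named "Shadow", labeled 影合わせ, shadow matching) built on a parent gimmick class.
; When given a guide Blueprint, it binds to that guide's ShadowCl event and calls Clear when it fires, unbinding on guide reset.
; A SetDebug function can write the gimmick label to a debug text widget, but nothing in the graph runs it.
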(event `self.ReceiveBeginPlay`
  (`parent.ReceiveBeginPlay`)
  (set `self.Name` "Shadow"))

(event `カスタムイベント_0`
  (`self.Clear`))

(event `Get_Guide`
  (params (Guid :type "/Game/Asset/BP/BP_Guide Object Reference"))
  (bind _output_get (set `self.BP_Guid` Guid))
  (add `/Game/Asset/BP/BP_Guide.shadow_Cl` _output_get (delegate `カスタムイベント_0`)))

(event `Reset_Guide`
  (remove `/Game/Asset/BP/BP_Guide.shadow_Cl` (`self.BP_Guid`) (delegate `カスタムイベント_0`)))

(fn `Set_Debug`
  (bind _asdebug_mozi (cast `/Game/Asset/BP/Gimmick/Debug_mozi` (`WidgetComponent.GetUserWidgetObject` (`self.Widget`))))
  (`TextBlock.SetText` (`/Game/Asset/BP/Gimmick/Debug_mozi.TextBlock_439` _asdebug_mozi) "影合わせ"))

(fn `UserConstructionScript`
  (`parent.UserConstructionScript`))