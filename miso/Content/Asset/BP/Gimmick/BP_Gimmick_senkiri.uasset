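; BP_Gimmick_senkiri is the line-cutting (線切り) gimmick, which hosts a BP_Cut child actor as its puzzle.
; On BeginPlay it binds that actor's OnClear event to Cleared, which calls Clear to report the gimmick as solved.
; It also writes the gimmick's label to a Debug_mozi widget and sets its Name to "Senkiri".
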(event `self.ReceiveBeginPlay`
  (`parent.ReceiveBeginPlay`)
  (bind _asbp_cut (cast `/Game/Asset/BP/BP_Cut` (`ChildActorComponent.ChildActor` (`self.BP_Cut`))))
  (add `/Game/Asset/BP/BP_Cut.OnClear` _asbp_cut (delegate `Cleared`))
  (bind _asdebug_mozi (cast `/Game/Asset/BP/Gimmick/Debug_mozi` (`WidgetComponent.GetUserWidgetObject` (`self.Widget`))))
  (`TextBlock.SetText` (`/Game/Asset/BP/Gimmick/Debug_mozi.TextBlock_439` _asdebug_mozi) "線切り")
  (set `self.Name` "Senkiri"))

(event `Cleared`
  (`self.Clear`))

(fn `UserConstructionScript`
  (`parent.UserConstructionScript`))