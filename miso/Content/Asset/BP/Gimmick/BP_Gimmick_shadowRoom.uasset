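; Shadow-room gimmick Blueprint, labelled "影合わせ" (shadow matching) in its debug display, with a rotatable camera.
; On BeginPlay it writes that label into the Debug_mozi user widget held by its widget component.
; UpdateCamera adds X to the camera's world pitch and Y to its yaw, keeping roll; nothing in this file calls it.
; No shadow-matching logic appears in these graphs, and Tick and overlap events are disabled.
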(event `self.ReceiveBeginPlay`
  (`parent.ReceiveBeginPlay`)
  (`self.Set_Debug`))

(fn `Set_Debug`
  (bind _asdebug_mozi (cast `/Game/Asset/BP/Gimmick/Debug_mozi` (`WidgetComponent.GetUserWidgetObject` (`self.Widget`))))
  (`TextBlock.SetText` (`/Game/Asset/BP/Gimmick/Debug_mozi.TextBlock_439` _asdebug_mozi) "影合わせ"))

(fn `UpdateCamera`
  (params (X :type "Float (double-precision)") (Y :type "Float (double-precision)"))
  (bind _camera (`self.Camera`))
  (`SceneComponent.K2_SetWorldRotation` _camera (`KismetMathLibrary.MakeRotator` (.roll (`SceneComponent.K2_GetComponentRotation` _camera)) (+ (.pitch (`SceneComponent.K2_GetComponentRotation` _camera)) X) (+ (.yaw (`SceneComponent.K2_GetComponentRotation` _camera)) Y)) false false))

(fn `UserConstructionScript`
  (`parent.UserConstructionScript`))