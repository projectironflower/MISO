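; Balance scale (tenbin) gimmick that wraps a Balance child actor and reports when it is cleared.
; On BeginPlay it casts the child actor to Balance, binds to its OnClear event and sets the gimmick's name.
; When that event fires, it calls Clear to mark the gimmick as cleared.
; SetDebug is an empty stub, and its debug-text widget code is disconnected.
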(event `self.ReceiveBeginPlay`
  (`parent.ReceiveBeginPlay`)
  (bind _asbalance (cast `/Game/Asset/BP/Balance` (`ChildActorComponent.ChildActor` (`self.Balance`))))
  (add `/Game/Asset/BP/Balance.OnClear` _asbalance (delegate `Cleared`))
  (set `self.Name` "Balance"))

(event `Cleared`
  (`self.Clear`))

(fn `Set_Debug`)

(fn `UserConstructionScript`
  (`parent.UserConstructionScript`))