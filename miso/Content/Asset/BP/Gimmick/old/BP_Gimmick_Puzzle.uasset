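; Puzzle gimmick actor that wraps a BP_Puzzle_ child actor and counts as cleared when that puzzle is cleared.
; On BeginPlay it sets a debug widget label to "パズル" (Puzzle), binds to the child's OnClear to call Clear, and sets its Name.
; A dynamic material change on the Cabinet mesh is present but never runs.
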(event `self.ReceiveBeginPlay`
  (`parent.ReceiveBeginPlay`)
  (`self.Set_Debug`)
  (bind _asbp_puzzle_ (cast `/Game/Asset/BP/BP_Puzzle_` (`ChildActorComponent.ChildActor` (`self.BP_Puzzle_`))))
  (add `/Game/Asset/BP/BP_Puzzle_.OnClear` _asbp_puzzle_ (delegate `Cleared`))
  (set `self.Name` "Puzzle"))

(event `Cleared`
  (`self.Clear`))

(fn `Set_Debug`
  (bind _asdebug_mozi (cast `/Game/Asset/BP/Gimmick/Debug_mozi` (`WidgetComponent.GetUserWidgetObject` (`self.Widget`))))
  (`TextBlock.SetText` (`/Game/Asset/BP/Gimmick/Debug_mozi.TextBlock_439` _asdebug_mozi) "パズル"))

(fn `UserConstructionScript`
  (`parent.UserConstructionScript`))