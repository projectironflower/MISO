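; Door Blueprint that slides open when the first-person character enters its trigger volume and closes when the character leaves.
; Overlap events play and reverse a single timeline, whose DoorPosition track drives relative-location lerps on two meshes, DoorSmallA and StaticMesh, between stored endpoint vectors.
; Movement is unswept, and an AddAudioComponent node is present but never executed.
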(event `self.ReceiveTick`
  (params (DeltaSeconds :type "Float (single-precision)")))

(event `self.Trigger.OnComponentBeginOverlap`
  (params (OverlappedComponent :type "PrimitiveComponent Object Reference") (OtherActor :type "Actor Object Reference") (OtherComp :type "PrimitiveComponent Object Reference") (OtherBodyIndex :type Integer) (bFromSweep :type Boolean) (SweepResult :type "HitResult Structure (by ref)"))
  (cast `/Game/Human/FirstPersonBP/Blueprints/FirstPersonCharacter` OtherActor)
  (bind (_direction _doorposition) (`Timeline|Timeline_0` :!label _label)
    (:`Update`
      (`SceneComponent.K2_SetRelativeLocation` (`self.Door_Small_A`) (`KismetMathLibrary.VLerp` (`self.DoorClosed`) (`self.DoorOpen`) _doorposition) false false)
      (`SceneComponent.K2_SetRelativeLocation` (`self.StaticMesh`) (`KismetMathLibrary.VLerp` (`self.NewVar_0`) (`self.new`) _doorposition) false false))))

(event `self.Trigger.OnComponentEndOverlap`
  (params (OverlappedComponent :type "PrimitiveComponent Object Reference") (OtherActor :type "Actor Object Reference") (OtherComp :type "PrimitiveComponent Object Reference") (OtherBodyIndex :type Integer))
  (cast `/Game/Human/FirstPersonBP/Blueprints/FirstPersonCharacter` OtherActor)
  (goto _label :!via `Reverse`))

(fn `UserConstructionScript`)