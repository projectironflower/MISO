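; Lockable sliding door that opens when the FirstPersonCharacter enters its trigger and closes when they leave.
; Trigger overlaps play or reverse a timeline, which lerps the door between closed and open positions only while unlocked.
; An audio component is added once as movement starts, and the Sound function re-arms it after the door opens past a threshold and fully closes.
; Tick runs that check and swaps the panel material to show lock state.
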(event `self.ReceiveTick`
  (params (DeltaSeconds :type "Float (single-precision)"))
  (bind _door_small_ui (`self.Door_Small_UI`))
  (`self.Sound`
    (:` `
      (if (`self.is_lock`)
        (`PrimitiveComponent.SetMaterial` _door_small_ui 0 "/Game/Asset/Map/MaterialInstance/MI_Door_Locked.MI_Door_Locked")
        (else
          (`PrimitiveComponent.SetMaterial` _door_small_ui 0 "/Game/Asset/Map/MaterialInstance/MI_Door_Unlocked.MI_Door_Unlocked"))))))

(event `self.Trigger.OnComponentBeginOverlap`
  (params (OverlappedComponent :type "PrimitiveComponent Object Reference") (OtherActor :type "Actor Object Reference") (OtherComp :type "PrimitiveComponent Object Reference") (OtherBodyIndex :type Integer) (bFromSweep :type Boolean) (SweepResult :type "HitResult Structure (by ref)"))
  (cast `/Game/Human/FirstPersonBP/Blueprints/FirstPersonCharacter` OtherActor)
  (bind (_direction _doorposition) (`Timeline|Timeline_0` :!label _label)
    (:`Update`
      (if (not (`self.is_lock`))
        (if (not (`self.is_sound`))
          (`AddComponent|NODE_AddAudioComponent-1`)
          (set `self.is_sound` true))
        (`SceneComponent.K2_SetRelativeLocation` (`self.Door_Small_A`) (`KismetMathLibrary.VLerp` (`self.DoorClosed`) (`self.DoorOpen`) _doorposition) false false)))))

(event `self.Trigger.OnComponentEndOverlap`
  (params (OverlappedComponent :type "PrimitiveComponent Object Reference") (OtherActor :type "Actor Object Reference") (OtherComp :type "PrimitiveComponent Object Reference") (OtherBodyIndex :type Integer))
  (cast `/Game/Human/FirstPersonBP/Blueprints/FirstPersonCharacter` OtherActor)
  (goto _label :!via `Reverse`))

(fn `UserConstructionScript`)