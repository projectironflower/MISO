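; Color-sequence puzzle actor made of four BP_ColorSwitch child actors: red, green, blue and yellow.
; The construction script positions each switch and assigns its material and number.
; Each switch event waits briefly, then pushes its number onto a stack, which is checked against CorrectNumber at three entries.
; A match calls CallOnClear and deactivates the switches; a mismatch reverses all four and empties the stack.
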(event `self.ReceiveBeginPlay`
  (bind _asbp_color_switch (cast `/Game/Asset/BP/BP_ColorSwitch` (`ChildActorComponent.ChildActor` (`self.Red`))))
  (add `/Game/Asset/BP/BP_ColorSwitch.OnSwitch` _asbp_color_switch (delegate `OnRed`))
  (bind _asbp_color_switch_2 (cast `/Game/Asset/BP/BP_ColorSwitch` (`ChildActorComponent.ChildActor` (`self.Green`))))
  (add `/Game/Asset/BP/BP_ColorSwitch.OnSwitch` _asbp_color_switch_2 (delegate `OnGreen`))
  (bind _asbp_color_switch_3 (cast `/Game/Asset/BP/BP_ColorSwitch` (`ChildActorComponent.ChildActor` (`self.Blue`))))
  (add `/Game/Asset/BP/BP_ColorSwitch.OnSwitch` _asbp_color_switch_3 (delegate `OnBlue`))
  (bind _asbp_color_switch_4 (cast `/Game/Asset/BP/BP_ColorSwitch` (`ChildActorComponent.ChildActor` (`self.Yellow`))))
  (add `/Game/Asset/BP/BP_ColorSwitch.OnSwitch` _asbp_color_switch_4 (delegate `OnYellow`)))

(event `OnRed`
  (`KismetSystemLibrary.Delay` 0.5)
  (`self.AddStack` 0))

(event `OnGreen`
  (`KismetSystemLibrary.Delay` 0.5)
  (`self.AddStack` 1))

(event `OnBlue`
  (`KismetSystemLibrary.Delay` 0.5)
  (`self.AddStack` 2))

(event `OnYellow`
  (`KismetSystemLibrary.Delay` 0.5)
  (`self.AddStack` 3))

(fn `AddStack`
  (params (num :type Integer))
  (bind _stack (`self.Stack`))
  (`KismetArrayLibrary.Array_Add` _stack num)
  (if (== (`KismetArrayLibrary.Array_Length` _stack) 3)
    (`self.CheckAnswer`)))

(fn `CheckAnswer`
  (for _index (range 3)
    (if (not (== (`|GetArrayItem` (`self.Stack`) _index) (`|GetArrayItem` (`self.CorrectNumber`) _index)))
      (`self.Reset`)
      (return)))
  (`self.OnClear`)
  (`self.SetDisable`))

(fn `Reset`
  (bind _stack (`self.Stack`))
  (bind _asbp_color_switch (cast `/Game/Asset/BP/BP_ColorSwitch` (`ChildActorComponent.ChildActor` (`self.Red`))))
  (`/Game/Asset/BP/BP_ColorSwitch.Reverse` _asbp_color_switch)
  (bind _asbp_color_switch_2 (cast `/Game/Asset/BP/BP_ColorSwitch` (`ChildActorComponent.ChildActor` (`self.Green`))))
  (`/Game/Asset/BP/BP_ColorSwitch.Reverse` _asbp_color_switch_2)
  (bind _asbp_color_switch_3 (cast `/Game/Asset/BP/BP_ColorSwitch` (`ChildActorComponent.ChildActor` (`self.Blue`))))
  (`/Game/Asset/BP/BP_ColorSwitch.Reverse` _asbp_color_switch_3)
  (bind _asbp_color_switch_4 (cast `/Game/Asset/BP/BP_ColorSwitch` (`ChildActorComponent.ChildActor` (`self.Yellow`))))
  (`/Game/Asset/BP/BP_ColorSwitch.Reverse` _asbp_color_switch_4)
  (`KismetArrayLibrary.Array_Clear` _stack)
  (`KismetArrayLibrary.Array_Resize` _stack))

(fn `SetCorrectNumber`)

(fn `SetDisable`
  (bind _asbp_color_switch (cast `/Game/Asset/BP/BP_ColorSwitch` (`ChildActorComponent.ChildActor` (`self.Red`))))
  (set `/Game/Asset/BP/BP_ColorSwitch.IsActive` false _asbp_color_switch)
  (bind _asbp_color_switch_2 (cast `/Game/Asset/BP/BP_ColorSwitch` (`ChildActorComponent.ChildActor` (`self.Green`))))
  (set `/Game/Asset/BP/BP_ColorSwitch.IsActive` false _asbp_color_switch_2)
  (bind _asbp_color_switch_3 (cast `/Game/Asset/BP/BP_ColorSwitch` (`ChildActorComponent.ChildActor` (`self.Blue`))))
  (set `/Game/Asset/BP/BP_ColorSwitch.IsActive` false _asbp_color_switch_3)
  (bind _asbp_color_switch_4 (cast `/Game/Asset/BP/BP_ColorSwitch` (`ChildActorComponent.ChildActor` (`self.Yellow`))))
  (set `/Game/Asset/BP/BP_ColorSwitch.IsActive` false _asbp_color_switch_4))

(fn `UserConstructionScript`
  (`SceneComponent.K2_SetRelativeLocation` (`self.Red`) (`self.PositionRed`) false false)
  (`SceneComponent.K2_SetRelativeLocation` (`self.Green`) (`self.PositionGreen`) false false)
  (`SceneComponent.K2_SetRelativeLocation` (`self.Blue`) (`self.PositionBlue`) false false)
  (`SceneComponent.K2_SetRelativeLocation` (`self.Yellow`) (`self.PositionYellow`) false false)
  (bind _asbp_color_switch (cast `/Game/Asset/BP/BP_ColorSwitch` (`ChildActorComponent.ChildActor` (`self.Red`))))
  (`PrimitiveComponent.SetMaterial` (`/Game/Asset/BP/BP_ColorSwitch.Mesh` _asbp_color_switch) 0 "/Engine/EngineDebugMaterials/VertexColorViewMode_RedOnly.VertexColorViewMode_RedOnly")
  (set `/Game/Asset/BP/BP_ColorSwitch.Number` 0 _asbp_color_switch)
  (bind _asbp_color_switch_2 (cast `/Game/Asset/BP/BP_ColorSwitch` (`ChildActorComponent.ChildActor` (`self.Green`))))
  (`PrimitiveComponent.SetMaterial` (`/Game/Asset/BP/BP_ColorSwitch.Mesh` _asbp_color_switch_2) 0 "/Engine/EngineDebugMaterials/VertexColorViewMode_GreenOnly.VertexColorViewMode_GreenOnly")
  (set `/Game/Asset/BP/BP_ColorSwitch.Number` 1 _asbp_color_switch_2)
  (bind _asbp_color_switch_3 (cast `/Game/Asset/BP/BP_ColorSwitch` (`ChildActorComponent.ChildActor` (`self.Blue`))))
  (`PrimitiveComponent.SetMaterial` (`/Game/Asset/BP/BP_ColorSwitch.Mesh` _asbp_color_switch_3) 0 "/Engine/EngineDebugMaterials/VertexColorViewMode_BlueOnly.VertexColorViewMode_BlueOnly")
  (set `/Game/Asset/BP/BP_ColorSwitch.Number` 2 _asbp_color_switch_3)
  (bind _asbp_color_switch_4 (cast `/Game/Asset/BP/BP_ColorSwitch` (`ChildActorComponent.ChildActor` (`self.Yellow`))))
  (`PrimitiveComponent.SetMaterial` (`/Game/Asset/BP/BP_ColorSwitch.Mesh` _asbp_color_switch_4) 0 "/Engine/EditorMaterials/WidgetMaterial_Current.WidgetMaterial_Current")
  (set `/Game/Asset/BP/BP_ColorSwitch.Number` 3 _asbp_color_switch_4))