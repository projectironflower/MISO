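; Sound box actor with three hit targets (right, center, left) that play three audio components in an order shuffled at BeginPlay.
; Hitting a target stops all sounds and plays its own; area overlaps also stop sounds and update IsArea flags.
; GetName and GetIndex match sounds to mizu, kaze or hono by display name.
; SetIndex picks the visible panel and material index, reapplied every Tick through newly created dynamic material instances.
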(event `self.ReceiveBeginPlay`
  (bind _p_center (`self.P_center`))
  (bind _p_right (`self.p_right`))
  (bind _p_reft (`self.P_reft`))
  (bind _sound (`self.sound`))
  (`KismetArrayLibrary.Array_Shuffle` (`self.index`))
  (bind _returnvalue (`AddComponent|NODE_AddAudioComponent-0`))
  (`KismetArrayLibrary.Array_Add` _sound _returnvalue)
  (bind _returnvalue_2 (`AddComponent|NODE_AddAudioComponent-1`))
  (`KismetArrayLibrary.Array_Add` _sound _returnvalue_2)
  (bind _returnvalue_3 (`AddComponent|NODE_AddAudioComponent-2`))
  (`KismetArrayLibrary.Array_Add` _sound _returnvalue_3)
  (`self.Set_Draw` :!label _label)
  (bind _returnvalue_4 (`PrimitiveComponent.CreateDynamicMaterialInstance` _p_reft 0 (`PrimitiveComponent.GetMaterial` _p_reft 0) "index"))
  (`MaterialInstanceDynamic.SetScalarParameterValue` _returnvalue_4 "index" (`self.m_index`))
  (bind _returnvalue_5 (`PrimitiveComponent.CreateDynamicMaterialInstance` _p_center 0 (`PrimitiveComponent.GetMaterial` _p_center 0) "index"))
  (`MaterialInstanceDynamic.SetScalarParameterValue` _returnvalue_5 "index" (`self.m_index`))
  (bind _returnvalue_6 (`PrimitiveComponent.CreateDynamicMaterialInstance` _p_right 0 (`PrimitiveComponent.GetMaterial` _p_right 0) "index"))
  (`MaterialInstanceDynamic.SetScalarParameterValue` _returnvalue_6 "index" (`self.m_index`)))

(event `self.ReceiveActorBeginOverlap`
  (params (OtherActor :type "Actor Object Reference")))

(event `self.ReceiveTick`
  (params (DeltaSeconds :type "Float (single-precision)"))
  (goto _label))

(event `self.right.OnComponentHit`
  (params (HitComponent :type "PrimitiveComponent Object Reference") (OtherActor :type "Actor Object Reference") (OtherComp :type "PrimitiveComponent Object Reference") (NormalImpulse :type "Vector Structure") (Hit :type "HitResult Structure (by ref)"))
  (`self.Stop_Sound`)
  (`AudioComponent.Play` (`|GetArrayItem` (`self.sound`) (`|GetArrayItem` (`self.index`))) 0.0))

(event `self.center.OnComponentHit`
  (params (HitComponent :type "PrimitiveComponent Object Reference") (OtherActor :type "Actor Object Reference") (OtherComp :type "PrimitiveComponent Object Reference") (NormalImpulse :type "Vector Structure") (Hit :type "HitResult Structure (by ref)"))
  (`self.Stop_Sound`)
  (`AudioComponent.Play` (`|GetArrayItem` (`self.sound`) (`|GetArrayItem` (`self.index`) 1)) 0.0))

(event `self.reft.OnComponentHit`
  (params (HitComponent :type "PrimitiveComponent Object Reference") (OtherActor :type "Actor Object Reference") (OtherComp :type "PrimitiveComponent Object Reference") (NormalImpulse :type "Vector Structure") (Hit :type "HitResult Structure (by ref)"))
  (`self.Stop_Sound`)
  (`AudioComponent.Play` (`|GetArrayItem` (`self.sound`) (`|GetArrayItem` (`self.index`) 2)) 0.0))

(event `self.C_right.OnComponentBeginOverlap`
  (params (OverlappedComponent :type "PrimitiveComponent Object Reference") (OtherActor :type "Actor Object Reference") (OtherComp :type "PrimitiveComponent Object Reference") (OtherBodyIndex :type Integer) (bFromSweep :type Boolean) (SweepResult :type "HitResult Structure (by ref)"))
  (`self.Stop_Sound`)
  (`KismetArrayLibrary.Array_Set` (`self.is_Area`) 0 true))

(event `self.C_right.OnComponentEndOverlap`
  (params (OverlappedComponent :type "PrimitiveComponent Object Reference") (OtherActor :type "Actor Object Reference") (OtherComp :type "PrimitiveComponent Object Reference") (OtherBodyIndex :type Integer))
  (`self.Stop_Sound`)
  (`KismetArrayLibrary.Array_Set` (`self.is_Area`)))

(event `self.C_Center.OnComponentBeginOverlap`
  (params (OverlappedComponent :type "PrimitiveComponent Object Reference") (OtherActor :type "Actor Object Reference") (OtherComp :type "PrimitiveComponent Object Reference") (OtherBodyIndex :type Integer) (bFromSweep :type Boolean) (SweepResult :type "HitResult Structure (by ref)"))
  (`self.Stop_Sound`)
  (`KismetArrayLibrary.Array_Set` (`self.is_Area`) 1 true))

(event `self.C_Center.OnComponentEndOverlap`
  (params (OverlappedComponent :type "PrimitiveComponent Object Reference") (OtherActor :type "Actor Object Reference") (OtherComp :type "PrimitiveComponent Object Reference") (OtherBodyIndex :type Integer))
  (`self.Stop_Sound`)
  (`KismetArrayLibrary.Array_Set` (`self.is_Area`) 1))

(event `self.C_left.OnComponentBeginOverlap`
  (params (OverlappedComponent :type "PrimitiveComponent Object Reference") (OtherActor :type "Actor Object Reference") (OtherComp :type "PrimitiveComponent Object Reference") (OtherBodyIndex :type Integer) (bFromSweep :type Boolean) (SweepResult :type "HitResult Structure (by ref)"))
  (`self.Stop_Sound`)
  (`KismetArrayLibrary.Array_Set` (`self.is_Area`) 2 true))

(event `self.C_left.OnComponentEndOverlap`
  (params (OverlappedComponent :type "PrimitiveComponent Object Reference") (OtherActor :type "Actor Object Reference") (OtherComp :type "PrimitiveComponent Object Reference") (OtherBodyIndex :type Integer))
  (`self.Stop_Sound`)
  (`KismetArrayLibrary.Array_Set` (`self.is_Area`) 2))

(fn `Get_index`
  (params (string :type String))
  (returns (Index :type Integer))
  (`|ExecutionSequence`
    (:`then_0`
      (if (`KismetStringLibrary.Contains` (`KismetSystemLibrary.GetDisplayName` (`|GetArrayItem` (`self.sound`) (`|GetArrayItem` (`self.index`)))) string)
        (return 0)))
    (:`then_1`
      (if (`KismetStringLibrary.Contains` (`KismetSystemLibrary.GetDisplayName` (`|GetArrayItem` (`self.sound`) (`|GetArrayItem` (`self.index`) 1))) string)
        (return 1)))
    (:`then_2`
      (if (`KismetStringLibrary.Contains` (`KismetSystemLibrary.GetDisplayName` (`|GetArrayItem` (`self.sound`) (`|GetArrayItem` (`self.index`) 2))) string)
        (return 2)))))

(fn `Get_Name`
  (params (index :type Integer))
  (returns (string :type String))
  (bind _returnvalue (`KismetSystemLibrary.GetDisplayName` (`|GetArrayItem` (`self.sound`) (`|GetArrayItem` (`self.index`) index))))
  (if (`KismetStringLibrary.Contains` _returnvalue "mizu")
    (set `self.string` "mizu"))
  (if (`KismetStringLibrary.Contains` _returnvalue "kaze")
    (set `self.string` "kaze"))
  (if (`KismetStringLibrary.Contains` _returnvalue "hono")
    (set `self.string` "hono"))
  (return (`self.string`)))

(fn `Set_Draw`
  (switch `int` (`self.Draw_index`)
    (:`1`
      (`SceneComponent.SetVisibility` (`self.p_right`) true false)
      (`SceneComponent.SetVisibility` (`self.P_center`) false false)
      (`SceneComponent.SetVisibility` (`self.P_reft`) false false))
    (:`2`
      (`SceneComponent.SetVisibility` (`self.p_right`) false false)
      (`SceneComponent.SetVisibility` (`self.P_center`) true false)
      (`SceneComponent.SetVisibility` (`self.P_reft`) false false))
    (:`3`
      (`SceneComponent.SetVisibility` (`self.p_right`) false false)
      (`SceneComponent.SetVisibility` (`self.P_center`) false false)
      (`SceneComponent.SetVisibility` (`self.P_reft`) true false))))

(fn `Set_index`
  (params (Material :type "Float (double-precision)") (Pos :type Integer))
  (set `self.m_index` Material)
  (set `self.Draw_index` Pos))

(fn `Stop_Sound`
  (for _index (range 3)
    (`AudioComponent.Stop` (`|GetArrayItem` (`self.sound`) _index))))

(fn `UserConstructionScript`)