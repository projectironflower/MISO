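; BP_C is an actor Blueprint that lets the player toggle a WBP_S widget on screen with the 4 key.
; On BeginPlay it enables input from player controller 0 and creates and stores one WBP_S instance.
; Each press of 4 runs a FlipFlop that alternately adds the widget to the viewport with the mouse cursor shown, or removes it and hides the cursor.
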(event `self.ReceiveBeginPlay`
  (`self.EnableInput` (`GameplayStatics.GetPlayerController` 0))
  (bind _returnvalue (`|CreateWidget` "/Game/Asset/Widget/WBP_S.WBP_S_C"))
  (set `self.C` _returnvalue))

(event `Key|Four`
  (params (Key :type "Key Structure"))
  (bind _returnvalue (`GameplayStatics.GetPlayerController` 0))
  (bind _c (`self.C`))
  (:`Pressed`
    (`/Engine/EditorBlueprintResources/StandardMacros.FlipFlop`
      (:`A`
        (`UserWidget.AddToViewport` _c 0)
        (set `PlayerController.bShowMouseCursor` true _returnvalue))
      (:`B`
        (`Widget.RemoveFromParent` _c)
        (set `PlayerController.bShowMouseCursor` false _returnvalue)))))

(fn `UserConstructionScript`)