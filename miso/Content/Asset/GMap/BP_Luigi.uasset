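; BP_Luigi sets up a randomized three-stage sound puzzle with Left, Center and Right choices per stage.
; On BeginPlay it shuffles three audio components across each stage and sends a random panel index to all nine choices.
; Judge functions then leave one choice per stage non-warping.
; The first follows sound placement, the second the panel index, and the third the sound at the second stage's non-warp slot.
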(event `self.ReceiveBeginPlay`
  (`self.Set_Sound`
    (:` `
      (`self.Set_Panel`)
      (`self.Fast_Judge`)
      (`self.Second_Judge`)
      (`self.Third_Judge`))))

(event `self.ReceiveTick`
  (params (DeltaSeconds :type "Float (single-precision)")))

(fn `Get_index`
  (params (Name :type String :default "hono"))
  (returns (index :type Integer))
  (locals (SoundIndex :type Integer))
  (bind _sound (`self.Sound`))
  (if (`KismetStringLibrary.Contains` (`KismetSystemLibrary.GetDisplayName` (`|GetArrayItem` _sound)) Name)
    (set `local.SoundIndex` 0)
    (return (`local.SoundIndex`))
    (elif (`KismetStringLibrary.Contains` (`KismetSystemLibrary.GetDisplayName` (`|GetArrayItem` _sound 1)) Name)
      (set `local.SoundIndex` 1)
      (return (`local.SoundIndex`))
      (elif (`KismetStringLibrary.Contains` (`KismetSystemLibrary.GetDisplayName` (`|GetArrayItem` _sound 2)) Name)
        (set `local.SoundIndex` 2)
        (return (`local.SoundIndex`))))))

(fn `UserConstructionScript`)