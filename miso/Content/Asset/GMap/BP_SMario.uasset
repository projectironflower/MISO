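; Sound-quiz answer spot that plays MSound while the player is inside SoundArea and judges them on entering JudgmentArea.
; A spot flagged IsWarp plays a wrong-answer sound, moves the player to the Warp's Y and briefly pulses IsDoor.
; Otherwise it plays the correct sound and sets IsCheck, so Tick holds IsDoor true.
; The construction script offsets and scales both areas, and BeginPlay writes its number to a widget.
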(event `self.ReceiveBeginPlay`
  (bind _asnuber (cast `/Game/Asset/GMap/nuber` (`WidgetComponent.GetUserWidgetObject` (`self.Widget`))))
  (`TextBlock.SetText` (`/Game/Asset/GMap/nuber.Nnber_Text` _asnuber) (`self.Nunber`)))

(event `self.ReceiveTick`
  (params (DeltaSeconds :type "Float (single-precision)"))
  (if (`self.Is_Check`)
    (set `self.Is_Door` true)))

(event `self.JudgmentArea.OnComponentBeginOverlap`
  (params (OverlappedComponent :type "PrimitiveComponent Object Reference") (OtherActor :type "Actor Object Reference") (OtherComp :type "PrimitiveComponent Object Reference") (OtherBodyIndex :type Integer) (bFromSweep :type Boolean) (SweepResult :type "HitResult Structure (by ref)"))
  ;[1 1 1] プレイヤーの移動/判定サウンド再生
  (set `self.Is_Judge` true)
  (`self.Judment` OtherActor)
  (set `self.Is_Judge` false))

(event `self.SoundArea.OnComponentBeginOverlap`
  (params (OverlappedComponent :type "PrimitiveComponent Object Reference") (OtherActor :type "Actor Object Reference") (OtherComp :type "PrimitiveComponent Object Reference") (OtherBodyIndex :type Integer) (bFromSweep :type Boolean) (SweepResult :type "HitResult Structure (by ref)"))
  ;[1 1 1] 音の再生、ストップ
  (if (== (`GameplayStatics.GetPlayerCharacter` 0) OtherActor)
    (`AudioComponent.Play` (`self.M_Sound`) 0.0)))

(event `self.SoundArea.OnComponentEndOverlap`
  (params (OverlappedComponent :type "PrimitiveComponent Object Reference") (OtherActor :type "Actor Object Reference") (OtherComp :type "PrimitiveComponent Object Reference") (OtherBodyIndex :type Integer))
  ;[1 1 1] 音の再生、ストップ
  (if (== (`GameplayStatics.GetPlayerCharacter` 0) OtherActor)
    (`AudioComponent.Stop` (`self.M_Sound`))))

(fn `Get_Sound`
  (returns (Sound_Name :type String))
  (return (`KismetSystemLibrary.GetDisplayName` (`AudioComponent.Sound` (`self.M_Sound`)))))

(fn `Set_Panel_Pos`
  (params (index :type Integer))
  (bind _plane (`self.Plane`))
  (switch `int` index
    (:`0`
      (`SceneComponent.K2_AddLocalOffset` _plane (200.0 0.0 0.0) false false))
    (:`1`
      (`SceneComponent.K2_AddLocalOffset` _plane (0.0 0.0 0.0) false false))
    (:`2`
      (`SceneComponent.K2_AddLocalOffset` _plane (-200.0 0.0 0.0) false false)))
  (return))

(fn `Set_Sound`
  (params (M_Sound :type "AudioComponent Object Reference"))
  (set `self.M_Sound` M_Sound)
  (return))

(fn `UserConstructionScript`
  (`self.Set_JidgArea`)
  (`self.Set_SoundArea`))