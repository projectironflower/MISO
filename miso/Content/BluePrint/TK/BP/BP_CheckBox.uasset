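; BP_CheckBox is an actor that runs a four-slot check puzzle through a WBP_Check widget.
; On BeginPlay it enables player input, creates the widget and fills its four text slots from T01 to T04.
; Tick compares each slot's check state against its expected value and sets the widget's IsClear only when all four match.
; The 2 key toggles the widget and mouse cursor.
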(event `self.ReceiveBeginPlay`
  (bind _check (`self.Check`))
  (`self.EnableInput` (`GameplayStatics.GetPlayerController` 0))
  (bind _returnvalue (`|CreateWidget` "/Game/BluePrint/TK/BP/WBP_Check.WBP_Check_C"))
  (set `self.Check` _returnvalue)
  (`/Game/BluePrint/TK/BP/WBP_Check.Set_Text` _check 1 (`self.T_01`))
  (`/Game/BluePrint/TK/BP/WBP_Check.Set_Text` _check 2 (`self.T_02`))
  (`/Game/BluePrint/TK/BP/WBP_Check.Set_Text` _check 3 (`self.T_03`))
  (`/Game/BluePrint/TK/BP/WBP_Check.Set_Text` _check 4 (`self.T_04`)))

(event `self.ReceiveTick`
  (params (DeltaSeconds :type "Float (single-precision)"))
  (bind _check (`self.Check`))
  (bind _check_2 (`self.Check`))
  (bind _check_3 (`self.Check`))
  (bind _check_4 (`self.Check`))
  (bind _returnvalue (`/Game/BluePrint/TK/BP/WBP_Check.Get_Check` _check_4 1))
  (if (== _returnvalue (`self.01`))
    (bind _returnvalue_2 (`/Game/BluePrint/TK/BP/WBP_Check.Get_Check` _check 2))
    (if (== _returnvalue_2 (`self.02`))
      (bind _returnvalue_3 (`/Game/BluePrint/TK/BP/WBP_Check.Get_Check` _check_2 3))
      (if (== _returnvalue_3 (`self.03`))
        (bind _returnvalue_4 (`/Game/BluePrint/TK/BP/WBP_Check.Get_Check` (`self.Check`) 4))
        (if (== _returnvalue_4 (`self.04`))
          (set `/Game/BluePrint/TK/BP/WBP_Check.Is_Clear` true _check_3)
          (else
            (set `/Game/BluePrint/TK/BP/WBP_Check.Is_Clear` false _check_3)))
        (else
          (set `/Game/BluePrint/TK/BP/WBP_Check.Is_Clear` false _check_2)))
      (else
        (set `/Game/BluePrint/TK/BP/WBP_Check.Is_Clear` false _check)))
    (else
      (set `/Game/BluePrint/TK/BP/WBP_Check.Is_Clear` false _check_4))))

(event `Key|Two`
  (params (Key :type "Key Structure"))
  (bind _returnvalue (`GameplayStatics.GetPlayerController` 0))
  (bind _check (`self.Check`))
  (:`Pressed`
    (`/Engine/EditorBlueprintResources/StandardMacros.FlipFlop`
      (:`A`
        (`UserWidget.AddToViewport` _check 0)
        (set `PlayerController.bShowMouseCursor` true _returnvalue))
      (:`B`
        (`Widget.RemoveFromParent` _check)
        (set `PlayerController.bShowMouseCursor` false _returnvalue)))))

(fn `UserConstructionScript`)