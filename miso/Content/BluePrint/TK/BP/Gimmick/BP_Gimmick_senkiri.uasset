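; BP_Gimmick_senkiri is a gimmick actor that wraps a BP_Cut child actor and reports when it is cleared.
; On BeginPlay it runs the parent logic, casts the BPCut child actor to BP_Cut and binds to its OnClear event.
; When that event fires, the gimmick calls its own OnClear, so the cutting logic itself stays in BP_Cut.
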(event `self.ReceiveBeginPlay`
  (`parent.ReceiveBeginPlay`)
  (bind _asbp_cut (cast `/Game/BluePrint/TK/BP/BP_Cut` (`ChildActorComponent.ChildActor` (`self.BP_Cut`))))
  (add `/Game/BluePrint/TK/BP/BP_Cut.OnClear` _asbp_cut (delegate `Cleared`)))

(event `Cleared`
  (`self.OnClear`))

(fn `UserConstructionScript`
  (`parent.UserConstructionScript`))