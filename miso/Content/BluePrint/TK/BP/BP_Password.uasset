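; Password puzzle actor that compares input from an on-screen keyboard widget against its Pass string.
; On BeginPlay it enables input and creates WBP_keyboard; the 1 key toggles the widget and mouse cursor.
; Tick polls the widget's IsEnter flag, and a match shows "Complete！", sets IsClear and calls the OnClear dispatcher.
; Nothing here resets IsEnter, so OnClear can fire every frame while it stays true.
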(event `self.ReceiveBeginPlay`
  (`self.EnableInput` (`GameplayStatics.GetPlayerController` 0))
  (bind _returnvalue (`|CreateWidget` "/Game/BluePrint/TK/BP/WBP_keyboard.WBP_keyboard_C"))
  (set `self.Keyboard` _returnvalue))

(event `self.ReceiveTick`
  (params (DeltaSeconds :type "Float (single-precision)"))
  (if (`/Game/BluePrint/TK/BP/WBP_keyboard.is_Enter` (`self.Keyboard`))
    (if (`KismetStringLibrary.EqualEqual_StrStr` (`KismetStringLibrary.JoinStringArray` (`/Game/BluePrint/TK/BP/WBP_keyboard.Pass` (`self.Keyboard`)) "") (`self.Pass`))
      (`TextBlock.SetText` (`/Game/BluePrint/TK/BP/WBP_keyboard.Passwordテキストブロック` (`self.Keyboard`)) "Complete！")
      (set `/Game/BluePrint/TK/BP/WBP_keyboard.is_Clear` true (`self.Keyboard`))
      (`self.OnClear`))))

(event `Key|One`
  (params (Key :type "Key Structure"))
  (bind _returnvalue (`GameplayStatics.GetPlayerController` 0))
  (bind _keyboard (`self.Keyboard`))
  (:`Pressed`
    (`/Engine/EditorBlueprintResources/StandardMacros.FlipFlop`
      (:`A`
        (`UserWidget.AddToViewport` _keyboard 0)
        (set `PlayerController.bShowMouseCursor` true _returnvalue))
      (:`B`
        (`Widget.RemoveFromParent` _keyboard)
        (set `PlayerController.bShowMouseCursor` false _returnvalue)))))

(fn `UserConstructionScript`)