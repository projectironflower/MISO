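; BP_Player is a Strix-networked player actor that places the locally owned instance at the PlayerStart or OperatorStart tagged point, chosen by the game instance's IsPlayer flag.
; When replication sync begins it registers MyRPC as a Strix RPC.
; Pressing Enter in the player role sends MyRPC to the other members, who show a W_Help widget on screen alongside debug prints.
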(event `self.ReceiveBeginPlay`
  (if (`StrixReplicatorComponent.GetIsOwner` (`self.StrixReplicator`))
    (bind _newparam (`/Game/BluePrint/Nishimaki/Network/GameInstance/FLIB_GINetwork.Get GI_Network`))
    (if (`/Game/BluePrint/Nishimaki/Network/GameInstance/GI_Network.IsPlayer` _newparam)
      (bind _outactors (`GameplayStatics.GetAllActorsWithTag` "PlayerStart"))
      (`self.K2_SetActorLocation` (`self.K2_GetActorLocation` (`|GetArrayItem` _outactors)))
      (else
        (bind _outactors_2 (`GameplayStatics.GetAllActorsWithTag` "OperatorStart"))
        (`self.K2_SetActorLocation` (`self.K2_GetActorLocation` (`|GetArrayItem` _outactors_2)))))))

(event `self.StrixReplicator.OnSyncBegin`
  (`StrixBlueprintFunctionLibrary.RegisterStrixRpc` self "MyRPC"))

(event `Key|Enter`
  (params (Key :type "Key Structure"))
  (:`Pressed`
    (bind _newparam (`/Game/BluePrint/Nishimaki/Network/GameInstance/FLIB_GINetwork.Get GI_Network`))
    (if (`/Game/BluePrint/Nishimaki/Network/GameInstance/GI_Network.IsPlayer` _newparam)
      (`KismetSystemLibrary.PrintString` "Send MyRPC" true true (struct :`G` 0.66 :`B` 1.0 :`A` 1.0) 5.0)
      (`StrixBlueprintFunctionLibrary.SendRpcToOtherMembers` self "MyRPC"))))

(fn `MyRPC`
  (`KismetSystemLibrary.PrintString` "Called MyRPC" true true (struct :`G` 0.66 :`B` 1.0 :`A` 1.0) 5.0)
  (bind _returnvalue (`|CreateWidget` "/Game/Sample/Widgets/W_Help.W_Help_C" (`GameplayStatics.GetPlayerController` 0)))
  (`UserWidget.AddToViewport` _returnvalue 0))

(fn `UserConstructionScript`)