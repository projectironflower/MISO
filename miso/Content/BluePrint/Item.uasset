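; Item is a pickup actor meant to be collected with the PickUp input action when the player is near.
; It enables input from player 0 on BeginPlay, and each press branches on DistanceCompare, destroying the item on true and printing debug strings either way.
; DistanceCompare contains a pawn-to-item distance threshold check and its string conversion, but neither expression is shown wired to its return values.
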(event `self.ReceiveBeginPlay`
  (`self.EnableInput` (`GameplayStatics.GetPlayerController` 0)))

(event `InputAction|PickUp`
  (params (Key :type "Key Structure"))
  (bind (_returnvalue _returnvalue2) (`self.DistanceCompare`))
  (:`Pressed`
    (if _returnvalue
      (`self.K2_DestroyActor`)
      (`KismetSystemLibrary.PrintString` _returnvalue2)
      (`KismetSystemLibrary.PrintString` "Destoroy")
      (else
        (`KismetSystemLibrary.PrintString` _returnvalue2)))))

(fn `UserConstructionScript`)