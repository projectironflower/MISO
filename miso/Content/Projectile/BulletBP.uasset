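; BulletBP is a projectile Actor that damages ThirdPersonCharacters in a game networked with Strix.
; It destroys itself five seconds after BeginPlay or on any Hit.
; Overlapping a ThirdPersonCharacter other than its instigator also destroys it.
; That overlap calls TakeDamage only where the victim's StrixReplicator is the owner, so the victim's owning client applies the damage.
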(event `self.ReceiveBeginPlay`
  (`KismetSystemLibrary.Delay` 5.0)
  (`self.K2_DestroyActor`))

(event `self.ReceiveActorBeginOverlap`
  (params (OtherActor :type "Actor Object Reference"))
  (bind _asthird_person_character (cast `/Game/ThirdPersonBP/Blueprints/ThirdPersonCharacter` OtherActor))
  (if (!= OtherActor (`self.GetInstigator`))
    (`self.K2_DestroyActor`)
    (if (`StrixReplicatorComponent.IsOwner` (`/Game/ThirdPersonBP/Blueprints/ThirdPersonCharacter.StrixReplicator` _asthird_person_character))
      (`/Game/ThirdPersonBP/Blueprints/ThirdPersonCharacter.TakeDamage` _asthird_person_character))))

(event `self.ReceiveHit`
  (params (MyComp :type "PrimitiveComponent Object Reference") (Other :type "Actor Object Reference") (OtherComp :type "PrimitiveComponent Object Reference") (bSelfMoved :type Boolean) (HitLocation :type "Vector Structure") (HitNormal :type "Vector Structure") (NormalImpulse :type "Vector Structure") (Hit :type "HitResult Structure (by ref)"))
  (`self.K2_DestroyActor`))

(fn `UserConstructionScript`)