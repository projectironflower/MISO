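; BP_Password is an actor that shows and hides a B_keyboard widget, apparently for password entry.
; BeginPlay enables input, creates the widget and copies the actor's Pass value into its Answer.
; Enter and Backspace set or clear IsView and the mouse cursor.
; Tick polls IsView every frame, calling AddToViewport or RemoveFromParent each time rather than only on change.
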(event `self.ReceiveBeginPlay`
  (`self.EnableInput` (`GameplayStatics.GetPlayerController` 0))
  (bind _returnvalue (`|CreateWidget` "/Game/BluePrint/TK/mistook/B_keyboard.B_keyboard_C"))
  (bind _output_get (set `self.Kyeboard` _returnvalue))
  (set `/Game/BluePrint/TK/mistook/B_keyboard.Answer` (`self.Pass`) _output_get))

(event `self.ReceiveTick`
  (params (DeltaSeconds :type "Float (single-precision)"))
  (bind _kyeboard (`self.Kyeboard`))
  (if (`self.is_View`)
    (`UserWidget.AddToViewport` _kyeboard 0)
    (else
      (`Widget.RemoveFromParent` _kyeboard))))

(event `Key|Enter`
  (params (Key :type "Key Structure"))
  (:`Pressed`
    (set `self.is_View` true)
    (set `PlayerController.bShowMouseCursor` true (`GameplayStatics.GetPlayerController` 0))))

(event `Key|BackSpace`
  (params (Key :type "Key Structure"))
  (:`Pressed`
    (set `self.is_View` false)
    (set `PlayerController.bShowMouseCursor` false (`GameplayStatics.GetPlayerController` 0))))

(fn `UserConstructionScript`)