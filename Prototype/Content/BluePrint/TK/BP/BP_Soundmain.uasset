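; BP_Soundmain is the manager for what appears to be a fire/wind/water (Hono/Kaze/Mizu) sound-matching puzzle across three SoundBoxes.
; BeginPlay gives each box a material number and one shared random position.
; Tick checks each box's area flags against its element name or that position, printing "あたり" (hit) and playing Atari on every matching frame.
; The "はずれ" (miss) feedback with Hazure is never wired.
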(event `self.ReceiveBeginPlay`
  (bind _pos (`self.Pos`))
  (set `self.Pos` (`KismetMathLibrary.RandomIntegerInRange` 1 3))
  (`/Game/BluePrint/TK/BP/BP_SoundBox.Set_index` (`|GetArrayItem` (`self.SoundBox`)) 1.0 _pos)
  (`/Game/BluePrint/TK/BP/BP_SoundBox.Set_index` (`|GetArrayItem` (`self.SoundBox`) 1) 2.0 _pos)
  (`/Game/BluePrint/TK/BP/BP_SoundBox.Set_index` (`|GetArrayItem` (`self.SoundBox`) 2) 3.0 _pos))

(event `self.ReceiveTick`
  (params (DeltaSeconds :type "Float (single-precision)"))
  (bind _output (`|GetArrayItem` (`self.SoundBox`)))
  (`|ExecutionSequence`
    (:`then_0`
      (bind _string (`/Game/BluePrint/TK/BP/BP_SoundBox.Get_Name` _output 0))
      (switch `string` _string
        (:`hono`
          (if (`self.Get_bool` 0 2)
            (`KismetSystemLibrary.PrintString` "あたり" true true (struct :`G` 0.66 :`B` 1.0 :`A` 1.0) (`GameplayStatics.GetWorldDeltaSeconds`) :!label _label)
            (`GameplayStatics.PlaySound2D` "/Game/BluePrint/TK/SE/atari.atari" 1.0 1.0 0.0 null null)))
        (:`kaze`
          (if (`self.Get_bool` 0 1)
            (goto _label)))
        (:`mizu`
          (bind _index (`/Game/BluePrint/TK/BP/BP_SoundBox.Get_index` _output "hono"))
          (if (`|GetArrayItem` (`/Game/BluePrint/TK/BP/BP_SoundBox.is_Area` _output) _index)
            (goto _label)))))
    (:`then_1`
      (switch `int` (`self.Pos`)
        (:`1`
          (if (`self.Get_bool` 1 1)
            (`KismetSystemLibrary.PrintString` "あたり" :!label _label_2)
            (`GameplayStatics.PlaySound2D` "/Game/BluePrint/TK/SE/atari.atari" 1.0 1.0 0.0 null null)))
        (:`2`
          (if (`self.Get_bool` 1 2)
            (goto _label_2)))
        (:`3`
          (if (`self.Get_bool` 1)
            (goto _label_2)))))
    (:`then_2`
      (bind _string_2 (`/Game/BluePrint/TK/BP/BP_SoundBox.Get_Name` (`|GetArrayItem` (`self.SoundBox`) 1) (`self.Pos`)))
      (switch `string` _string_2
        (:`hono`
          (if (`self.Get_bool` 2)
            (`KismetSystemLibrary.PrintString` "あたり" :!label _label_3)
            (`GameplayStatics.PlaySound2D` "/Game/BluePrint/TK/SE/atari.atari" 1.0 1.0 0.0 null null)))
        (:`kaze`
          (if (`self.Get_bool` 2 1)
            (goto _label_3)))
        (:`mizu`
          (if (`self.Get_bool` 2 2)
            (goto _label_3)))))))

(fn `UserConstructionScript`)