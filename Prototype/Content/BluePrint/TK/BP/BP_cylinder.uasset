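; BP_cylinder is a cylinder actor that can appear whole or cut and takes one of three colors.
; Each Tick reads IsCut, which SetCut writes, and shows either the whole Cylinder mesh or the two piece meshes, Cylinder1 and Cylinder2.
; SetColor maps an index to a blue, green or red material on all three meshes and stores it in Color.
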(event `self.ReceiveBeginPlay`)

(event `self.ReceiveTick`
  (params (DeltaSeconds :type "Float (single-precision)"))
  (if (`self.is_cut`)
    (`SceneComponent.SetVisibility` (`self.Cylinder`) false false)
    (`SceneComponent.SetVisibility` (`self.Cylinder1`) true false)
    (`SceneComponent.SetVisibility` (`self.Cylinder2`) true false)
    (else
      (`SceneComponent.SetVisibility` (`self.Cylinder1`) false false)
      (`SceneComponent.SetVisibility` (`self.Cylinder2`) false false)
      (`SceneComponent.SetVisibility` (`self.Cylinder`) true false))))

(fn `SetColor`
  (params (num :type Integer))
  (bind _cylinder (`self.Cylinder`))
  (switch `int` num
    (:`0`
      (`PrimitiveComponent.SetMaterial` _cylinder 0 "/Game/BluePrint/Kobayashi/Squares/Material/BlueMat.BlueMat")
      (`PrimitiveComponent.SetMaterial` (`self.Cylinder2`) 0 "/Game/BluePrint/Kobayashi/Squares/Material/BlueMat.BlueMat")
      (`PrimitiveComponent.SetMaterial` (`self.Cylinder1`) 0 "/Game/BluePrint/Kobayashi/Squares/Material/BlueMat.BlueMat")
      (set `self.Color` 0))
    (:`1`
      (`PrimitiveComponent.SetMaterial` _cylinder 0 "/Game/BluePrint/Kobayashi/Squares/Material/GreenMat.GreenMat")
      (`PrimitiveComponent.SetMaterial` (`self.Cylinder2`) 0 "/Game/BluePrint/Kobayashi/Squares/Material/GreenMat.GreenMat")
      (`PrimitiveComponent.SetMaterial` (`self.Cylinder1`) 0 "/Game/BluePrint/Kobayashi/Squares/Material/GreenMat.GreenMat")
      (set `self.Color` 1))
    (:`2`
      (`PrimitiveComponent.SetMaterial` _cylinder 0 "/Game/BluePrint/Kobayashi/Squares/Material/RedMat.RedMat")
      (`PrimitiveComponent.SetMaterial` (`self.Cylinder2`) 0 "/Game/BluePrint/Kobayashi/Squares/Material/RedMat.RedMat")
      (`PrimitiveComponent.SetMaterial` (`self.Cylinder1`) 0 "/Game/BluePrint/Kobayashi/Squares/Material/RedMat.RedMat")
      (set `self.Color` 2))))

(fn `SetCut`
  (params (bool :type Boolean))
  (set `self.is_cut` bool))

(fn `UserConstructionScript`)