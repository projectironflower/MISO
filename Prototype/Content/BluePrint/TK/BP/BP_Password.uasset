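; BP_Password is an actor that runs a password-entry check through an on-screen keyboard widget.
; On BeginPlay it enables input and creates a WBP_keyboard, which the 1 key toggles in the viewport along with the mouse cursor.
; Tick polls the widget's IsEnter flag, joins its entered Pass array and compares it to the actor's Pass.
; A match displays a completion message and sets the widget's IsClear flag.
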(event `self.ReceiveBeginPlay`
  (`self.EnableInput` (`GameplayStatics.GetPlayerController` 0))
  (bind _returnvalue (`|CreateWidget` "/Game/BluePrint/TK/BP/WBP_keyboard.WBP_keyboard_C"))
  (set `self.Kyeboard` _returnvalue))

(event `self.ReceiveTick`
  (params (DeltaSeconds :type "Float (single-precision)"))
  (if (`/Game/BluePrint/TK/BP/WBP_keyboard.is_Enter` (`self.Kyeboard`))
    (if (`KismetStringLibrary.EqualEqual_StrStr` (`KismetStringLibrary.JoinStringArray` (`/Game/BluePrint/TK/BP/WBP_keyboard.Pass` (`self.Kyeboard`)) "") (`self.Pass`))
      (`TextBlock.SetText` (`/Game/BluePrint/TK/BP/WBP_keyboard.Passwordテキストブロック` (`self.Kyeboard`)) "Complete！")
      (set `/Game/BluePrint/TK/BP/WBP_keyboard.is_Clear` true (`self.Kyeboard`)))))

(event `Key|One`
  (params (Key :type "Key Structure"))
  (bind _returnvalue (`GameplayStatics.GetPlayerController` 0))
  (bind _kyeboard (`self.Kyeboard`))
  (:`Pressed`
    (`/Engine/EditorBlueprintResources/StandardMacros.FlipFlop`
      (:`A`
        (`UserWidget.AddToViewport` _kyeboard 0)
        (set `PlayerController.bShowMouseCursor` true _returnvalue))
      (:`B`
        (`Widget.RemoveFromParent` _kyeboard)
        (set `PlayerController.bShowMouseCursor` false _returnvalue)))))

(fn `UserConstructionScript`)