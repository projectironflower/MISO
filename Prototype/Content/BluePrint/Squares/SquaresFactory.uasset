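; Factory actor that spawns a 10x10 grid of Squares actors on BeginPlay, laying out a board from data tables.
; Spawn positions derive from the actor's location plus a scene component offset, with the Y index reversed along world X.
; GetTableData reads each cell from the table selected by TableDataIndex, using Y for the row and X for the column.
; That value, converted to SquaresStatus, drives each square's ChangeMaterial call.
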(event `self.ReceiveBeginPlay`
  (bind _square_x (`self.square_x`))
  (while (< _square_x 10)
    (while (< (`self.square_y`) 10)
      (bind _returnvalue (`|SpawnActorFromClass` "/Game/BluePrint/Squares/Squares.Squares_C" (`KismetMathLibrary.MakeTransform` (+ (`KismetMathLibrary.MakeVector` (* (- 9 (`self.square_y`)) 150.0) (* (`self.square_x`) 150.0)) (`self.K2_GetActorLocation`) (`SceneComponent.RelativeLocation` (`self.Scene`)))) "Undefined" "OverrideRootScale" null null))
      (bind _stateindex (`self.GetTableData` (`self.square_x`) (`self.square_y`) (`self.TableDataIndex`)))
      (`/Game/BluePrint/Squares/Squares.ChangeMaterial` _returnvalue (cast `/Game/BluePrint/Squares/Enum/SquaresStatus` _stateindex))
      (`/Engine/EditorBlueprintResources/StandardMacros.IncrementInt` (`self.square_y`)))
    (`/Engine/EditorBlueprintResources/StandardMacros.IncrementInt` _square_x
      (:`  `
        (set `self.square_y` 0)))))

(fn `GetTableData`
  (params (X :type Integer) (Y :type Integer) (TableDataIndex :type Integer))
  (returns (StateIndex :type Byte))
  (bind _returnvalue (`|GetDataTableRow` (`|GetArrayItem` (`self.DataTableArray`) TableDataIndex) (`self.GetRowName` Y))
    (:`then`
      (switch `int` X
        (:`0`
          (bind (_column_0 _column_1 _column_2 _column_3 _column_4 _column_5 _column_6 _column_7 _column_8 _column_9) (break `/Game/BluePrint/Squares/Structure/SquaresPatternTable` _returnvalue))
          (return _column_0))
        (:`1`
          (return _column_1))
        (:`2`
          (return _column_2))
        (:`3`
          (return _column_3))
        (:`4`
          (return _column_4))
        (:`5`
          (return _column_5))
        (:`6`
          (return _column_6))
        (:`7`
          (return _column_7))
        (:`8`
          (return _column_8))
        (:`9`
          (return _column_9))))))

(fn `UserConstructionScript`)